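; AC_Att is a character attribute component that handles XP gain and leveling.
; The Win_XP event adds earned XP and, when the threshold is reached, raises the level, scales the next threshold by a multiplier and restores life to maximum.
; Leftover XP is computed as threshold minus current XP, so any overshoot becomes negative, and each call grants at most one level.
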(event `Win_XP`
  (params (XP_Ganho :type Integer))
  (bind _current_levelup_xp (`self.Current_LevelUP_XP`))
  ;[1 1 1] HUD
  (bind _output_get (set `self.Current_XP` (+ XP_Ganho (`self.Current_XP`))))
  (if (>= _output_get (`self.Current_LevelUP_XP`))
    (set `self.Current_Level` (+ (`self.Current_Level`) 1))
    (set `self.Current_XP` (- _current_levelup_xp _output_get))
    (set `self.Current_LevelUP_XP` (* _current_levelup_xp 1.5))
    (set `self.Current_Life` (`self.Max_Life`))))