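; Gameplay game mode that spawns the player's chosen hero when the level begins.
; On BeginPlay it reads GeneroHero from GI_Chronicles to spawn either BP_PlayerGirl or BP_PlayerBoy at the PlayerStart, then possesses it.
; It then switches to game-only input with a hidden cursor, adds the default Enhanced Input mapping context and shows the HUD widget.
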(event `self.ReceiveBeginPlay`
  (bind _returnvalue (`GameplayStatics.GetPlayerController` 0))
  (bind _returnvalue_2 (`GameplayStatics.GetActorOfClass` "/Script/Engine.PlayerStart"))
  (bind _asgi_chronicles (cast `/Game/Chronicles/Blueprints/GI_Chronicles` (`GameplayStatics.GetGameInstance`)))
  (if (== (`/Game/Chronicles/Blueprints/GI_Chronicles.GeneroHero` _asgi_chronicles) 1)
    (bind _returnvalue_3 (`self.GetTransform` _returnvalue_2))
    (bind _returnvalue_4 (`|SpawnActorFromClass` "/Game/Chronicles/Characters/Players/BP_PlayerGirl.BP_PlayerGirl_C" _returnvalue_3 "Undefined" "MultiplyWithRoot" null null))
    (`Controller.Possess` _returnvalue _returnvalue_4)
    (else
      (bind _returnvalue_5 (`|SpawnActorFromClass` "/Game/Chronicles/Characters/Players/BP_PlayerBoy.BP_PlayerBoy_C" _returnvalue_3 "Undefined" "MultiplyWithRoot" null null))
      (`Controller.Possess` _returnvalue _returnvalue_5)))
  (`WidgetBlueprintLibrary.SetInputMode_GameOnly` _returnvalue)
  (set `PlayerController.bShowMouseCursor` false _returnvalue)
  (`EnhancedInputSubsystemInterface.AddMappingContext` (pcsubsystem `EnhancedInputLocalPlayerSubsystem` _returnvalue) "/Game/ThirdPerson/Input/IMC_Default.IMC_Default" 0 (struct))
  (bind _returnvalue_6 (`|CreateWidget` "/Game/Chronicles/HUD/WBP_HUD.WBP_HUD_C"))
  (`UserWidget.AddToViewport` _returnvalue_6 0))

(fn `UserConstructionScript`)