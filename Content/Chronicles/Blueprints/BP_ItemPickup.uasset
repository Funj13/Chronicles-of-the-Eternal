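; BP_ItemPickup is a world item that the player collects into the AC_Inventario inventory with the F key.
; On BeginPlay it looks up ItemID in DT_Items, but always assigns the MaterialSphere mesh.
; Character overlap shows a prompt with the row's name and quantity and enables input, which end overlap never disables.
; F adds the actor's own Quantidade, then destroys it or prints a full-inventory message.
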(event `self.ReceiveBeginPlay`
  (`self.InitializeItem`))

(event `self.InteractionArea.OnComponentBeginOverlap`
  (params (OverlappedComponent :type "PrimitiveComponent Object Reference") (OtherActor :type "Actor Object Reference") (OtherComp :type "PrimitiveComponent Object Reference") (OtherBodyIndex :type Integer) (bFromSweep :type Boolean) (SweepResult :type "HitResult Structure (by ref)"))
  (bind _pickupwidget (`self.PickupWidget`))
  ;[1 1 1] Coletar Item
  (cast `Character` OtherActor)
  (`SceneComponent.SetVisibility` _pickupwidget true false)
  (`self.EnableInput` (`GameplayStatics.GetPlayerController` 0))
  (bind _returnvalue (`|GetDataTableRow` "/Game/Chronicles/Date/DT_Items.DT_Items" (`self.ItemID`))
    (:`then`
      (bind _aswbp_pickup_prompt (cast `/Game/Chronicles/UI/Inventario/WBP_PickupPrompt` (`WidgetComponent.GetUserWidgetObject` _pickupwidget)))
      (bind (_itemid _nomeitem _descricao _quantidade) (break `ItemInventario` _returnvalue))
      (`/Game/Chronicles/UI/Inventario/WBP_PickupPrompt.SetItemInfo` _aswbp_pickup_prompt _nomeitem _quantidade))))

(event `Key|F`
  (params (Key :type "Key Structure"))
  ;[1 1 1] Tecla F
  (:`Pressed`
    (bind _returnvalue (`AC_Inventario.AdicionarItemPorID` (`self.GetComponentByClass` (`GameplayStatics.GetPlayerCharacter` 0) "/Script/Chlonicles.AC_Inventario") (`self.ItemID`) (`self.Quantidade`)))
    (if _returnvalue
      (`self.K2_DestroyActor`)
      (else
        (`KismetSystemLibrary.PrintString` "Inventário Cheio")))))

(event `self.InteractionArea.OnComponentEndOverlap`
  (params (OverlappedComponent :type "PrimitiveComponent Object Reference") (OtherActor :type "Actor Object Reference") (OtherComp :type "PrimitiveComponent Object Reference") (OtherBodyIndex :type Integer))
  ;[1 1 1] Sumir com o Item
  (cast `Character` OtherActor)
  (`SceneComponent.SetVisibility` (`self.PickupWidget`) false false))

(fn `InitializeItem`
  ;[1 1 1] Comentário
  (bind _returnvalue (`|GetDataTableRow` "/Game/Chronicles/Date/DT_Items.DT_Items" (`self.ItemID`))
    (:`then`
      (`StaticMeshComponent.SetStaticMesh` (`self.ItemMesh`) "/Game/StarterContent/Props/MaterialSphere.MaterialSphere")
      (set `self.Out Row` _returnvalue))))

(fn `UserConstructionScript`)